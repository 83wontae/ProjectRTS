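; Enemy spawn area actor that periodically spawns AI units around itself while its live count stays under a cap.
; Tick accumulates time toward the spawn interval and shows progress on a name-tag gauge, resetting it while the cap is reached.
; Each BP_Unit spawns at a random point on a ring, receiving its definition ID, hand weapon settings and faction.
; A destroyed-event binding decrements the count, reopening spawning.
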(event EventTick
  (params (DeltaSeconds :type Float%20%28single-precision%29))
  (Variables|Default|SetIsSpawning (CallFunction|IsCanSpawn))
  (if (Variables|Default|GetIsSpawning)
    (bind _output_get (Variables|Default|SetTotalDeltaSeconds (+ DeltaSeconds (Variables|Default|GetTotalDeltaSeconds))))
    (Default|SetGauge (Variables|Default|GetBP_ActorNameTagComponent) _output_get (Variables|Default|GetSpawnTime))
    (if (> (Variables|Default|GetTotalDeltaSeconds) (Variables|Default|GetSpawnTime))
      (CallFunction|SpawnUnit))
    (else
      (bind _output_get_2 (Variables|Default|SetTotalDeltaSeconds 0.0))
      (Default|SetGauge (Variables|Default|GetBP_ActorNameTagComponent) _output_get_2 (Variables|Default|GetSpawnTime)))))

(fn ConstructionScript)

(fn SpawnUnit
  (Variables|Default|SetTotalDeltaSeconds 0.0)
  (bind _returnvalue (AI|SpawnAIFromClass "/Game/ProjectRTS/Unit/BP_Unit.BP_Unit_C" "/Game/ProjectRTS/AI/BT_Unit.BT_Unit" (CallFunction|GetRandomRoundLocation 2e+02) "0, 0, 0" false 0))
  (bind _asbp_unit (Utilities|Casting|CastToBP_Unit _returnvalue))
  (Utilities|FlowControl|Sequence
    (:then_0
      (Variables|/Script/ProjectRTS.RtsUnitCharacter|SetUnitDefinitionId _asbp_unit (Variables|Default|GetUnit%20Definition%20Id)))
    (:then_1
      (bind _output_get (LocalVariables|SetEquipComp (Actor|GetComponentbyClass _asbp_unit "/Script/ProjectRTS.EquipComponent")))
      (Utilities|IsValid _output_get
        (:Is%20Valid
          (Variables|/Script/ProjectRTS.EquipComponent|SetRightHandSocketName (LocalVariables|GetEquipComp) (Variables|Default|GetR%20Weapon%20Row%20Name))
          (Variables|/Script/ProjectRTS.EquipComponent|SetLeftHandSocketName (LocalVariables|GetEquipComp) (Variables|Default|GetL%20Weapon%20Row%20Name)))))
    (:then_2
      (bind _output_get_2 (LocalVariables|SetStateComp (Actor|GetComponentbyClass _asbp_unit "/Script/ProjectRTS.StateComponent")))
      (Utilities|IsValid _output_get_2
        (:Is%20Valid
          (Variables|/Script/ProjectRTS.StateComponent|Setm_Faction (LocalVariables|GetStateComp) (Variables|Default|GetFaction)))))
    (:then_3
      (Game|BindEventtoOnDestroyed _asbp_unit (EventDispatchers|CreateEvent :!event EventDestroyedUnit))
      (Variables|Default|SetSpawnedUnitCnt (+ (Variables|Default|GetSpawnedUnitCnt) 1)))))

(fn GetRandomRoundLocation
  (params (Radius :type Float%20%28double-precision%29))
  (LocalVariables|SetRand%20Radian (Math|Trig|DegreesToRadians (Math|Random|RandomFloatinRange 0.0 3.6e+02)))
  (return (+ (Transformation|GetActorLocation) (Math|Vector|MakeVector (* (Math|Trig|Cos(Radians) (LocalVariables|GetRand%20Radian)) Radius) (* (Math|Trig|Sin(Radians) (LocalVariables|GetRand%20Radian)) Radius) 0.0) "0.000000,0.000000,80.000000")))

(fn EventDestroyedUnit
  (params (DestroyedActor :type Actor%20Object%20Reference))
  (Variables|Default|SetSpawnedUnitCnt (- (Variables|Default|GetSpawnedUnitCnt) 1)))

(fn IsCanSpawn
  (return (> (Variables|Default|GetMaxSpawnedUnits) (Variables|Default|GetSpawnedUnitCnt))))