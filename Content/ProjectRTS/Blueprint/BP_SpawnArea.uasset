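; BP_SpawnArea is a trigger zone that runs a repeating spawn timer while a player-controlled Character overlaps its box.
; Tick fills the name tag component's gauge toward SpawnTime, then calls SpawnUnit, and clears the timer when spawning is off.
; SpawnUnit resets the timer and reaches an empty authority switch, so no unit is created here.
; GetRandomRoundLocation computes a raised random point on a surrounding circle but is never called here.
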(event OnComponentBeginOverlap(Box)
  (params (OverlappedComponent :type Primitive%20Component%20Object%20Reference) (OtherActor :type Actor%20Object%20Reference) (OtherComp :type Primitive%20Component%20Object%20Reference) (OtherBodyIndex :type Integer) (bFromSweep :type Boolean) (SweepResult :type Hit%20Result%20Structure%20%28by%20ref%29))
  (bind _ascharacter (Utilities|Casting|CastToCharacter OtherActor))
  (if (Pawn|IsPlayerControlled _ascharacter)
    (Variables|Default|SetOverlapUnit _ascharacter)
    (Variables|Default|SetIsSpawning true)))

(event OnComponentEndOverlap(Box)
  (params (OverlappedComponent :type Primitive%20Component%20Object%20Reference) (OtherActor :type Actor%20Object%20Reference) (OtherComp :type Primitive%20Component%20Object%20Reference) (OtherBodyIndex :type Integer))
  (bind _ascharacter (Utilities|Casting|CastToCharacter OtherActor))
  (if (Pawn|IsPlayerControlled _ascharacter)
    (Variables|Default|SetOverlapUnit 0)
    (Variables|Default|SetIsSpawning false)))

(event EventTick
  (params (DeltaSeconds :type Float%20%28single-precision%29))
  (if (Variables|Default|GetIsSpawning)
    (bind _output_get (Variables|Default|SetTotalDeltaSeconds (+ DeltaSeconds (Variables|Default|GetTotalDeltaSeconds))))
    (Default|SetGauge (Variables|Default|GetBP_ActorNameTagComponent) _output_get (Variables|Default|GetSpawnTime))
    (if (> (Variables|Default|GetTotalDeltaSeconds) (Variables|Default|GetSpawnTime))
      (CallFunction|SpawnUnit))
    (else
      (bind _output_get_2 (Variables|Default|SetTotalDeltaSeconds 0.0))
      (Default|SetGauge (Variables|Default|GetBP_ActorNameTagComponent) _output_get_2 (Variables|Default|GetSpawnTime)))))

(fn ConstructionScript)

(fn SpawnUnit
  (Variables|Default|SetTotalDeltaSeconds 0.0)
  (Networking|SwitchHasAuthority))

(fn GetRandomRoundLocation
  (params (Radius :type Float%20%28double-precision%29))
  (LocalVariables|SetRand (Math|Random|RandomFloatinRange 0.0 3.6e+02))
  (return (+ (Transformation|GetActorLocation) (Math|Vector|MakeVector (* (Math|Trig|Cos(Radians) (* (LocalVariables|GetRand) 2.0 3.14)) Radius) (* (Math|Trig|Sin(Radians) (* (LocalVariables|GetRand) 2.0 3.14)) Radius) 0.0) "0.000000,0.000000,80.000000")))