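; BP_Unit1 is an RTS unit Blueprint with a name tag and a selection indicator.
; StateComp dispatchers for level, HP and XP changes update the name tag component, which takes the unit's display name and starts at level zero.
; The construction script makes the head mesh follow the main mesh's animation through a leader pose component.
; Selection events toggle the visibility of the selection decal.
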(event EventDispatcherUpdateHp(StateComp)
  (params (CurHp :type Float%20%28double-precision%29) (MaxHp :type Float%20%28double-precision%29))
  (Default|SetHp (Variables|Default|GetBP_UnitNameTagComponent) CurHp MaxHp))

(event EventDispatcherExpChanged(StateComp)
  (params (CurrentExp :type Float%20%28double-precision%29) (RequiredExp :type Float%20%28double-precision%29))
  (Default|SetXP (Variables|Default|GetBP_UnitNameTagComponent) CurrentExp RequiredExp))

(event EventDispatcherLevelUp(StateComp)
  (params (NewLevel :type Integer))
  (CallFunction|UpdateNameandLevel NewLevel))

(event EventBeginPlay
  (CallFunction|UpdateNameandLevel))

(fn ConstructionScript
  (Components|SkinnedMesh|SetLeaderPoseComponent (Variables|Default|GetHeadMesh) (Variables|Character|GetMesh) true true))

(fn EventUnitSelected
  (params (IsSelected :type Boolean))
  (Rendering|SetVisibility (Variables|Default|GetSelectionDecal) IsSelected true)
  (return false))

(fn UpdateNameandLevel
  (params (Level :type Integer))
  (Default|SetName (Variables|Default|GetBP_UnitNameTagComponent) Level (Utilities|GetDisplayName self)))