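; RTS player controller that handles unit selection and move orders, and creates the HUD widget on BeginPlay.
; Left click clears selection and adds the UnitInterface actor under the cursor, though it signals it with selected=false.
; Dragging past a minimum distance draws a HUD rectangle and selects enclosed units on release.
; Right click sends selected Characters to the cursor hit location via SimpleMoveToLocation on their controllers.
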(event Input|EnhancedActionEvents|EnhancedInputActionIA_ClickL
  (params (ActionValue :type Boolean) (ElapsedSeconds :type Float%20%28double-precision%29) (TriggeredSeconds :type Float%20%28double-precision%29) (InputAction :type Input%20Action%20Object%20Reference :default "/Game/ProjectRTS/Input/Actions/IA_ClickL.IA_ClickL"))
  (bind (_hitresult _returnvalue) (Game|Player|GetHitResultUnderCursorbyChannel "TraceTypeQuery1" true))
  (bind _hitactor (Collision|BreakHitResult _hitresult))
  (:Triggered
    (CallFunction|OnSelectionTriggered))
  (:Started
    (CallFunction|OnSelectionStarted)
    (CallFunction|UnSelectedAllUnits)
    (if _returnvalue
      (bind _asunit_interface (Utilities|Casting|CastToUnitInterface _hitactor))
      (Utilities|Array|Add (Variables|Default|GetSelectedActors) _hitactor)
      (Class|UnitInterface|EventUnitSelected _asunit_interface false)))
  (:Completed
    (CallFunction|OnSelectionCompleted)))

(event Input|EnhancedActionEvents|EnhancedInputActionIA_ClickR
  (params (ActionValue :type Boolean) (ElapsedSeconds :type Float%20%28double-precision%29) (TriggeredSeconds :type Float%20%28double-precision%29) (InputAction :type Input%20Action%20Object%20Reference :default "/Game/ProjectRTS/Input/Actions/IA_ClickR.IA_ClickR"))
  (bind (_hitresult _returnvalue) (Game|Player|GetHitResultUnderCursorbyChannel "TraceTypeQuery1" true))
  (bind _location (Collision|BreakHitResult _hitresult))
  (:Started
    (if _returnvalue
      (Development|PrintString (Utilities|String|ToString(Vector) _location))
      (CallFunction|MoveUnits _location))))

(event EventBeginPlay
  (bind _returnvalue (UserInterface|CreateWidget "/Game/ProjectRTS/Widget/HudWidget.HudWidget_C"))
  (bind _output_get (Variables|Default|SetHudWidget _returnvalue))
  (UserInterface|Viewport|AddtoViewport _output_get 0))

(event MouseInput|EventActorOnClicked
  (params (ButtonPressed :type Key%20Structure :default "None"))
  (Development|PrintString "ActorOnClicked!!!"))

(fn ConstructionScript)

(fn UnSelectedAllUnits
  (for _array_element (Variables|Default|GetSelectedActors)
    (bind _asunit_interface (Utilities|Casting|CastToUnitInterface _array_element))
    (Class|UnitInterface|EventUnitSelected _asunit_interface false))
  (Utilities|Array|Clear (Variables|Default|GetSelectedActors)))

(fn MoveUnits
  (params (Goal :type Vector%20%28by%20ref%29))
  (for _array_element (Variables|Default|GetSelectedActors)
    (bind _ascharacter (Utilities|Casting|CastToCharacter _array_element))
    (AI|Navigation|SimpleMovetoLocation (Pawn|GetController _ascharacter) Goal)))

(fn OnSelectionStarted
  (bind _self self)
  (bind (_locationx _locationy) (Class|WidgetLayoutLibrary|GetMousePositionScaledbyDPI _self))
  (Variables|Default|SetSelectionStartPosition (Math|Vector2D|MakeVector2D _locationx _locationy)))

(fn OnSelectionTriggered
  (bind _self self)
  (bind _hudwidget (Variables|Default|GetHudWidget))
  (bind (_locationx _locationy) (Class|WidgetLayoutLibrary|GetMousePositionScaledbyDPI _self))
  (if (> (Math|Vector|Distance2D(Vector) (Variables|Default|GetSelectionStartPosition) (Math|Vector2D|MakeVector2D _locationx _locationy)) (Variables|Default|GetDragDistanceMin))
    (Default|ShowSelectDragUI _hudwidget true)
    (Default|UpdateDrawSelectDragUI _hudwidget (Variables|Default|GetSelectionStartPosition) (Math|Vector2D|MakeVector2D _locationx _locationy))))

(fn OnSelectionCompleted
  (bind _self self)
  (bind _selectionstartposition (Variables|Default|GetSelectionStartPosition))
  (bind (_locationx _locationy) (Class|WidgetLayoutLibrary|GetMousePositionScaledbyDPI _self))
  (bind _returnvalue (Math|Vector2D|MakeVector2D _locationx _locationy))
  (if (> (Math|Vector|Distance2D(Vector) _selectionstartposition _returnvalue) (Variables|Default|GetDragDistanceMin))
    (CallFunction|UnSelectedAllUnits)
    (CallFunction|DoSelectUnits (Class|RtsPlayerController|GetActorsInsideDragRect "/Script/ProjectRTS.UnitInterface" _selectionstartposition _returnvalue))
    (Default|ShowSelectDragUI (Variables|Default|GetHudWidget) false)))

(fn DoSelectUnits
  (params (Actors :type Array%20of%20Actor%20Object%20References))
  (CallFunction|UnSelectedAllUnits)
  (bind _output_get (Variables|Default|SetSelectedActors Actors))
  (for _array_element _output_get
    (bind _asunit_interface (Utilities|Casting|CastToUnitInterface _array_element))
    (Class|UnitInterface|EventUnitSelected _asunit_interface true)))