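; Player controller for RTS battle mode that creates the HUD and routes Enhanced Input to unit selection, movement and placement confirmation.
; Select press clears selection; dragging past a minimum distance updates the HUD marquee, and release selects UnitInterface actors inside it.
; Single-unit selection also runs on every release.
; Move input traces under the cursor for MoveUnits; selection, move and placement logic live outside this graph, and place-cancel is empty.
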(event Input|EnhancedActionEvents|EnhancedInputActionIA_UnitSelect
  (params (ActionValue :type Boolean) (ElapsedSeconds :type Float%20%28double-precision%29) (TriggeredSeconds :type Float%20%28double-precision%29) (InputAction :type Input%20Action%20Object%20Reference :default "/Game/ProjectRTS/Input/Actions/IA_UnitSelect.IA_UnitSelect"))
  (:Triggered
    (CallFunction|OnSelectionTriggered))
  (:Started
    (CallFunction|OnSelectionStarted)
    (Class|RtsPlayerController|UnSelectedAllUnits))
  (:Completed
    (CallFunction|OnSelectionCompleted)
    (Class|RtsPlayerController|DoSelectUnitSingle)))

(event Input|EnhancedActionEvents|EnhancedInputActionIA_UnitMove
  (params (ActionValue :type Boolean) (ElapsedSeconds :type Float%20%28double-precision%29) (TriggeredSeconds :type Float%20%28double-precision%29) (InputAction :type Input%20Action%20Object%20Reference :default "/Game/ProjectRTS/Input/Actions/IA_UnitMove.IA_UnitMove"))
  (bind (_hitresult _returnvalue) (Game|Player|GetHitResultUnderCursorbyChannel "TraceTypeQuery1" true))
  (:Started
    (if _returnvalue
      (Class|RtsPlayerController|MoveUnits (.Location (Collision|BreakHitResult _hitresult))))))

(event Input|EnhancedActionEvents|EnhancedInputActionIA_PlaceOK
  (params (ActionValue :type Boolean) (ElapsedSeconds :type Float%20%28double-precision%29) (TriggeredSeconds :type Float%20%28double-precision%29) (InputAction :type Input%20Action%20Object%20Reference :default "/Game/ProjectRTS/Input/Actions/IA_PlaceOK.IA_PlaceOK"))
  (:Completed
    (Class|RtsPlayerController|ConfirmPlacement)))

(event Input|EnhancedActionEvents|EnhancedInputActionIA_PlaceCancel
  (params (ActionValue :type Boolean) (ElapsedSeconds :type Float%20%28double-precision%29) (TriggeredSeconds :type Float%20%28double-precision%29) (InputAction :type Input%20Action%20Object%20Reference :default "/Game/ProjectRTS/Input/Actions/IA_PlaceCancel.IA_PlaceCancel")))

(event EventBeginPlay
  (|CallParentFunction)
  (CallFunction|CreateHudWidget "/Game/ProjectRTS/Widget/WorldHudWidget.WorldHudWidget_C"))

(fn ConstructionScript)

(fn OnSelectionStarted
  (bind _self self)
  (bind (_locationx _locationy) (Class|WidgetLayoutLibrary|GetMousePositionScaledbyDPI _self))
  (Variables|Default|SetSelectionStartPosition (Math|Vector2D|MakeVector2D _locationx _locationy)))

(fn OnSelectionTriggered
  (bind _self self)
  (bind (_locationx _locationy) (Class|WidgetLayoutLibrary|GetMousePositionScaledbyDPI _self))
  (if (> (Math|Vector|Distance2D(Vector) (Variables|Default|GetSelectionStartPosition) (Math|Vector2D|MakeVector2D _locationx _locationy)) (Variables|Default|GetDragDistanceMin))
    (bind _asbattle_hud_widget (Utilities|Casting|CastToBattleHudWidget (Variables|Default|GetHudWidget)))
    (Default|ShowSelectDragUI _asbattle_hud_widget true)
    (Default|UpdateDrawSelectDragUI _asbattle_hud_widget (Variables|Default|GetSelectionStartPosition) (Math|Vector2D|MakeVector2D _locationx _locationy))))

(fn OnSelectionCompleted
  (bind _self self)
  (bind _selectionstartposition (Variables|Default|GetSelectionStartPosition))
  (bind (_locationx _locationy) (Class|WidgetLayoutLibrary|GetMousePositionScaledbyDPI _self))
  (bind _returnvalue (Math|Vector2D|MakeVector2D _locationx _locationy))
  (if (> (Math|Vector|Distance2D(Vector) _selectionstartposition _returnvalue) (Variables|Default|GetDragDistanceMin))
    (Class|RtsPlayerController|UnSelectedAllUnits)
    (Class|RtsPlayerController|DoSelectUnits (Class|RtsPlayerController|GetActorsInsideDragRect "/Script/ProjectRTS.UnitInterface" _selectionstartposition _returnvalue))
    (bind _asbattle_hud_widget (Utilities|Casting|CastToBattleHudWidget (Variables|Default|GetHudWidget)))
    (Default|ShowSelectDragUI _asbattle_hud_widget false)))

(fn CreateHudWidget
  (params (Class :type User%20Widget%20Class%20Reference))
  (Utilities|FlowControl|Sequence
    (:then_0
      (bind _hudwidget (Variables|Default|GetHudWidget)
        (:then
          (Widget|RemovefromParent _hudwidget))
        (:else)))
    (:then_1
      (bind _returnvalue (UserInterface|CreateWidget Class))
      (bind _output_get (Variables|Default|SetHudWidget _returnvalue))
      (UserInterface|Viewport|AddtoViewport _output_get 0))))