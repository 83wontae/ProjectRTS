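; BP_RtsGameMode is the RTS game mode that loads the save, streams levels and assigns teams.
; BeginPlay loads save Slot1 and streams in World_Level.
; LoadLevel looks up a DT_Level row, swaps the streamed level with blocking loads, creates that row's HUD, and spawns recruited units via RecruitmentComponent when entering Battle_Level.
; Each starting player receives an incrementing team index on its player state.
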(event Custom|LoadLevel
  (params (LevelRowName :type Name))
  (bind _returnvalue (Utilities|GetDataTableRow "/Game/ProjectRTS/Data/DT_Level.DT_Level" LevelRowName)
    (:then
      (Game|UnloadStreamLevel(byName) (Variables|Default|GetCurLoadedLevel) true)
      (Utilities|FlowControl|Sequence
        (:then_0
          (bind _asbp_rts_player_controller (Utilities|Casting|CastToBP_RtsPlayerController (Game|GetPlayerController 0)))
          (Default|CreateHudWidget _asbp_rts_player_controller (.HudClass (Utilities|Struct|BreakST_Level _returnvalue))))
        (:then_1
          (bind _output_get (Variables|Default|SetCurLoadedLevel (.LevelName (Utilities|Struct|BreakST_Level _returnvalue))))
          (Game|LoadStreamLevel(byName) _output_get true true)
          (CallFunction|InitLoadLevel))))))

(event EventBeginPlay
  (CallFunction|InitGame)
  (bind _output_get (Variables|Default|SetCurLoadedLevel "World_Level"))
  (Game|LoadStreamLevel(byName) _output_get true true))

(event EventHandleStartingNewPlayer
  (params (NewPlayer :type Player%20Controller%20Object%20Reference))
  (|CallParentFunction NewPlayer)
  (bind _asbp_rts_player_state (Utilities|Casting|CastToBP_RtsPlayerState (Variables|/Script/Engine.Controller|GetPlayerState NewPlayer)))
  (bind _teamindex (CallFunction|GenNewTeamIndex))
  (Default|SetTeamIndex _asbp_rts_player_state _teamindex))

(fn ConstructionScript)

(fn GenNewTeamIndex
  (bind _output_get (Variables|Default|SetGenTeamIndex (+ (Variables|Default|GetGenTeamIndex) 1)))
  (return _output_get))

(fn InitLoadLevel
  (Development|PrintString "InitLoadLevel")
  (if (== (Variables|Default|GetCurLoadedLevel) "Battle_Level")
    (Class|RecruitmentComponent|SpawnRecruitedUnits (Actor|GetComponentbyClass (Game|GetPlayerController 0) "/Script/ProjectRTS.RecruitmentComponent") "PlayerUnits" 5e+02)))

(fn InitGame
  (Class|RtsSaveSubsystem|LoadGame (Subsystems|GetRtsSaveSubsystem) "Slot1"))