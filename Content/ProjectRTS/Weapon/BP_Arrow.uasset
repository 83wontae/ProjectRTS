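; BP_Arrow is an RTS projectile launched by a suggested-velocity impulse on its physics sphere toward TargetLocation.
; Tick aligns it with its velocity in flight.
; Overlapping another-faction unit Character stops physics, attaches it to the mesh, and on authority applies damage; blocking hits also stop it.
; Stopped arrows are destroyed after an authority-side delay, or earlier by Tick if HitTarget is invalid or the instigator is dead or not a unit.
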(event OnComponentBeginOverlap(Sphere)
  (params (OverlappedComponent :type Primitive%20Component%20Object%20Reference) (OtherActor :type Actor%20Object%20Reference) (OtherComp :type Primitive%20Component%20Object%20Reference) (OtherBodyIndex :type Integer) (bFromSweep :type Boolean) (SweepResult :type Hit%20Result%20Structure%20%28by%20ref%29))
  (Utilities|IsHitEnemy OtherActor
    (:True
      (bind _ascharacter (Utilities|Casting|CastToCharacter OtherActor))
      (Physics|SetSimulatePhysics (Variables|Default|GetSphere) false)
      (Transformation|AttachComponentToComponent (Variables|/Script/Engine.Character|GetMesh _ascharacter) "None" "KeepWorld" "KeepWorld" "KeepWorld" true)
      (Networking|SwitchHasAuthority
        (:Authority
          (bind _output_get (Variables|Default|SetHitTarget OtherActor))
          (Game|Damage|ApplyDamage _output_get 1e+01 (Game|GetInstigatorController) self)
          (Utilities|FlowControl|Delay 3.0)
          (Actor|DestroyActor))))))

(event OnComponentHit(Sphere)
  (params (HitComponent :type Primitive%20Component%20Object%20Reference) (OtherActor :type Actor%20Object%20Reference) (OtherComp :type Primitive%20Component%20Object%20Reference) (NormalImpulse :type Vector :default "0, 0, 0") (Hit :type Hit%20Result%20Structure%20%28by%20ref%29))
  (Physics|SetSimulatePhysics (Variables|Default|GetSphere) false)
  (Networking|SwitchHasAuthority
    (:Authority
      (Utilities|FlowControl|Delay 3.0)
      (Actor|DestroyActor))))

(event EventBeginPlay
  (bind _asunit_interface (Utilities|Casting|CastToUnitInterface (Game|GetInstigator)))
  (Variables|Default|SetTeamIndex (Class|UnitInterface|GetFaction _asunit_interface))
  (Physics|AddImpulse (Variables|Default|GetSphere) (CallFunction|ComputeProjectileLaunch (Transformation|GetActorLocation) (Variables|Default|GetTarget%20Location) 1.2e+03) "None" false))

(event EventTick
  (params (DeltaSeconds :type Float%20%28single-precision%29))
  (if (Physics|IsSimulatingPhysics (Variables|Default|GetSphere) "None")
    (bind _returnvalue (Physics|GetPhysicsLinearVelocity (Variables|Default|GetSphere) "None"))
    (Transformation|SetActorRotation (Math|Rotator|MakeRotfromX _returnvalue))
    (else
      (Variables|Default|GetHitTarget
        (:then
          (bind _asunit_interface (Utilities|Casting|CastToUnitInterface (Game|GetInstigator))
            (:then
              (if (Class|UnitInterface|IsDeath _asunit_interface)
                (Actor|DestroyActor :!label _label)))
            (:CastFailed
              (goto _label))))
        (:else
          (goto _label))))))

(fn ConstructionScript)

(fn ComputeProjectileLaunch
  (params (StartLocation :type Vector) (TargetLocation :type Vector) (LaunchSpeed :type Float%20%28double-precision%29))
  (bind _tossvelocity (Class|GameplayStatics|BlueprintSuggestProjectileVelocity StartLocation TargetLocation LaunchSpeed 0.0 "DoNotTrace" (Variables|/Script/Engine.SphereComponent|GetSphereRadius (Variables|Default|GetSphere)) false false false))
  (return _tossvelocity))