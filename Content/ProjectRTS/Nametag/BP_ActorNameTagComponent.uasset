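; BP_ActorNameTagComponent is a component that gives its actor a name tag widget with a name and gauge in ProjectRTS.
; On BeginPlay it creates the widget with itself as the owning component reference, adds it to the viewport and initializes it with the attach parent's owner.
; SetName, SetGauge and InitActor forward to the widget, which is removed on EndPlay.
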(event EventBeginPlay
  (bind _returnvalue (UserInterface|CreateWidget "/Game/ProjectRTS/Nametag/ActorTagWidget.ActorTagWidget_C" 0 self))
  (bind _output_get (Variables|Default|SetNameTag _returnvalue))
  (UserInterface|Viewport|AddtoViewport _output_get 0)
  (CallFunction|InitActor (Components|GetOwner (Transformation|GetAttachParent))))

(event EventEndPlay
  (params (EndPlayReason :type EEndPlayReason%20Enum :default "Destroyed"))
  (Widget|RemovefromParent (Variables|Default|GetNameTag)))

(fn SetName
  (params (Name :type String))
  (Default|SetName (Variables|Default|GetNameTag) Name))

(fn SetGauge
  (params (CurGauge :type Float%20%28double-precision%29) (MaxGauge :type Float%20%28double-precision%29))
  (Default|SetGauge (Variables|Default|GetNameTag) CurGauge MaxGauge))

(fn InitActor
  (params (Actor :type Actor%20Object%20Reference))
  (Default|InitActor (Variables|Default|GetNameTag) Actor))